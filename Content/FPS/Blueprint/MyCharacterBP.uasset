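; First-person player character Blueprint that handles movement, look input, HUD creation and weapon equipping.
; BeginPlay adds the HUD widget to the viewport, then equips the base player weapon.
; EquipWeapon stores the weapon class, swaps it into the Weapon child actor component and initializes the spawned actor through the PlayerWeaponI interface.
; Input axes drive yaw-relative movement and controller pitch and yaw.
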(event `self.ReceiveBeginPlay`
  (`parent.ReceiveBeginPlay`)
  (bind _returnvalue (`|CreateWidget` "/Game/FPS/Blueprint/HUD/HUDWidgetBP.HUDWidgetBP_C"))
  (`UserWidget.AddToViewport` _returnvalue 0)
  (`self.Equip Weapon` "/Game/FPS/Blueprint/PlayerBaseWeaponBP.PlayerBaseWeaponBP_C"))

(event `Equip Weapon`
  (params (weapon :type "/Game/FPS/Blueprint/PlayerBaseWeaponBP Class Reference"))
  (bind _weapon (`self.Weapon`))
  (bind _childactor (`ChildActorComponent.ChildActor` _weapon))
  (bind _output_get (set `self.CurrentWeapon` weapon))
  (`ChildActorComponent.SetChildActorClass` _weapon _output_get)
  (if (`KismetSystemLibrary.DoesImplementInterface` _childactor "/Game/FPS/Blueprint/PlayerWeaponI.PlayerWeaponI_C")
    (message `/Game/FPS/Blueprint/PlayerWeaponI.initializeWeapon` _childactor)))

(event `InputAxis|moveForward`
  (params (AxisValue :type "Float (single-precision)"))
  (bind (_returnvalue_roll _returnvalue_pitch _returnvalue_yaw) (`KismetMathLibrary.BreakRotator` (`self.GetControlRotation`)))
  (`self.AddMovementInput` (`KismetMathLibrary.GetForwardVector` (`KismetMathLibrary.MakeRotator` 0.0 0.0 _returnvalue_yaw)) AxisValue))

(event `InputAxis|moveRight`
  (params (AxisValue :type "Float (single-precision)"))
  (bind (_returnvalue_roll _returnvalue_pitch _returnvalue_yaw) (`KismetMathLibrary.BreakRotator` (`self.GetControlRotation`)))
  (`self.AddMovementInput` (`KismetMathLibrary.GetRightVector` (`KismetMathLibrary.MakeRotator` 0.0 0.0 _returnvalue_yaw)) AxisValue))

(event `InputAxis|LookVertical`
  (params (AxisValue :type "Float (single-precision)"))
  (`self.AddControllerPitchInput` AxisValue))

(event `InputAxis|LookHorizontal`
  (params (AxisValue :type "Float (single-precision)"))
  (`self.AddControllerYawInput` AxisValue))

(fn `UserConstructionScript`
  (`parent.UserConstructionScript`))