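; Base FPS enemy that runs a behavior tree on its AI controller and displays as a directional 2D flipbook sprite in the 3D world.
; Each tick yaws the sprite toward the player camera, then, unless dead or paused, computes the player's angle relative to the enemy's facing.
; Dot products with forward and right vectors select one of eight views, and velocity picks the walk or idle flipbook.
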(event `self.ReceiveBeginPlay`
  (`parent.ReceiveBeginPlay`)
  (bind _asenemy_controller_aibp (cast `/Game/FPS/Blueprint/Enemy/AI/EnemyControllerAIBP` (`self.GetController`)))
  (`AIController.RunBehaviorTree` _asenemy_controller_aibp (`self.BehaviorTree`)))

(event `self.ReceiveTick`
  (params (DeltaSeconds :type "Float (single-precision)"))
  (`parent.ReceiveTick` DeltaSeconds)
  (`self.SpriteFacePlayer`
    (:`Out`
      (if (not (or (`self.isDead`) (`self.PauseAngleCalculation`)))
        (`self.GetEnemyAngle`
          (:`Out`
            (`self.CheckIfWalking`
              (:`Out`
                (`self.CalculateFlip`)))))))))

(fn `SetFlipbook`
  (params (Walk :type "PaperFlipbook Object Reference") (Iddle :type "PaperFlipbook Object Reference"))
  (if (`self.isWalking`)
    (`PaperFlipbookComponent.SetFlipbook` (`self.PaperFlipbook`) Walk)
    (else
      (`PaperFlipbookComponent.SetFlipbook` (`self.PaperFlipbook`) Iddle))))

(fn `UserConstructionScript`
  (`parent.UserConstructionScript`))